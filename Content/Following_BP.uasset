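; Enemy Blueprint that starts moving toward the player when it sees a pawn and dies from accumulated damage.
; PawnSensing triggers AI MoveTo with player controller 0, rather than its pawn, as the target actor.
; AnyDamage lowers Health and, below zero, clears IsTrue, destroys the actor and prints EnemyCount.
; The EnemyCount update subtracts zero, so never decrements, and its zero-count branch is empty.
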(event OnSeePawn(PawnSensing)
  (params (Pawn :type Pawn%20Object%20Reference))
  (AI|AIMoveTo self "0, 0, 0" (Game|GetPlayerController 0) 5.0 false))

(event Game|Damage|EventAnyDamage
  (params (Damage :type Float%20%28single-precision%29) (DamageType :type Damage%20Type%20Object%20Reference) (InstigatedBy :type Controller%20Object%20Reference) (DamageCauser :type Actor%20Object%20Reference))
  (Variables|Default|SetHealth (- (Variables|Default|GetHealth) Damage))
  (if (< (Variables|Default|GetHealth) 0.0)
    (Variables|Default|SetIs%20True false)
    (Actor|DestroyActor)
    (bind _output_get (Variables|Default|SetEnemyCount (Math|Float|Truncate (- (Variables|Default|GetEnemyCount) 0.0))))
    (Development|PrintString (Utilities|String|ToString(Integer) _output_get))
    (if (== (Variables|Default|GetEnemyCount) 0)
      _)))

(fn ConstructionScript)