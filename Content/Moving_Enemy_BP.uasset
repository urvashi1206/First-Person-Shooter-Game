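; Moving enemy actor that patrols back and forth along the world X axis and can be killed by damage.
; On BeginPlay it stores its location as the start and a point offset along X as the end.
; Two timelines lerp between these points, one playing forward and the other in reverse, each triggering the other in an endless loop.
; Incoming damage reduces Health, and the actor clears IsTrue and destroys itself once Health drops below zero.
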(event EventBeginPlay
  (bind _returnvalue (Transformation|GetActorLocation))
  (Variables|Default|SetStart (Math|Vector|MakeVector (.x _returnvalue) (.y _returnvalue) (.z _returnvalue)))
  (Variables|Default|SetEnd (Math|Vector|MakeVector (+ (.x _returnvalue) 1e+03) (.y _returnvalue) (.z _returnvalue)))
  (bind _move (Timeline|Timeline PlayFromStart)
    (:Update
      (Transformation|SetActorRelativeLocation (Math|Vector|Lerp(Vector) (Variables|Default|GetStart) (Variables|Default|GetEnd) _move)))
    (:Finished
      (bind _move_2 (Timeline|Timeline_0 ReverseFromEnd)
        (:Update
          (Transformation|SetActorRelativeLocation (Math|Vector|Lerp(Vector) (Variables|Default|GetStart) (Variables|Default|GetEnd) _move_2)))
        (:Finished
          (Timeline|Timeline PlayFromStart))))))

(event Game|Damage|EventAnyDamage
  (params (Damage :type Float%20%28single-precision%29) (DamageType :type Damage%20Type%20Object%20Reference) (InstigatedBy :type Controller%20Object%20Reference) (DamageCauser :type Actor%20Object%20Reference))
  (Variables|Default|SetHealth (- (Variables|Default|GetHealth) Damage))
  (if (< (Variables|Default|GetHealth) 0.0)
    (Variables|Default|SetIsTrue false)
    (Actor|DestroyActor)))

(fn ConstructionScript)