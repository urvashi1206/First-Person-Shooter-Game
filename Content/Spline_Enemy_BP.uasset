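; Enemy actor that travels along a level spline and dies when its health drops below zero.
; On BeginPlay it finds the first Spline_BP actor and plays a Movement timeline scaled by TimeToComplete.
; Each update lerps distance over the spline length to set world location and rotation from the spline.
; AnyDamage subtracts from Health and destroys the actor once it goes negative.
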(event Custom|Move%20Object
  (bind _spline_ref (Variables|Default|GetSpline%20Ref))
  (Components|Timeline|SetPlayRate (Variables|Default|GetMovement) (/ 1.0 (Variables|Default|GetTime%20to%20Complete)))
  (bind _move (Timeline|Movement Play)
    (:Update
      (Transformation|SetActorTransform (Math|Transform|MakeTransform (Spline|GetLocationatDistanceAlongSpline (Variables|/Game/Spline_BP.Spline_BP_C|GetSpline _spline_ref) (Math|Float|Lerp 0.0 (Spline|GetSplineLength (Variables|/Game/Spline_BP.Spline_BP_C|GetSpline (Variables|Default|GetSpline%20Ref))) _move) "World") (Spline|GetRotationatDistanceAlongSpline (Variables|/Game/Spline_BP.Spline_BP_C|GetSpline _spline_ref) (Math|Float|Lerp 0.0 (Spline|GetSplineLength (Variables|/Game/Spline_BP.Spline_BP_C|GetSpline (Variables|Default|GetSpline%20Ref))) _move) "World") "1.000000,1.000000,1.000000")))))

(event EventBeginPlay
  (bind _returnvalue (Actor|GetActorOfClass "/Game/Spline_BP.Spline_BP_C"))
  (Variables|Default|SetSpline%20Ref _returnvalue)
  (CallFunction|MoveObject))

(event Game|Damage|EventAnyDamage
  (params (Damage :type Float%20%28single-precision%29) (DamageType :type Damage%20Type%20Object%20Reference) (InstigatedBy :type Controller%20Object%20Reference) (DamageCauser :type Actor%20Object%20Reference))
  (Variables|Default|SetHealth (- (Variables|Default|GetHealth) Damage))
  (if (< (Variables|Default|GetHealth) 0.0)
    (Variables|Default|SetIs%20True false)
    (Actor|DestroyActor)))

(fn ConstructionScript)