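; Spawn_BP is a pawn that pursues the player and can be killed by damage.
; On BeginPlay it issues a single AI MoveTo toward the player's BP_FirstPersonCharacter.
; AnyDamage subtracts from Health, and once Health drops below zero it sets IsTrue and destroys the actor.
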(event EventBeginPlay
  (bind _asbp_first_person_character (Utilities|Casting|CastToBP_FirstPersonCharacter (Game|GetPlayerCharacter 0)))
  (AI|AIMoveTo self "0, 0, 0" _asbp_first_person_character 5.0 false))

(event Game|Damage|EventAnyDamage
  (params (Damage :type Float%20%28single-precision%29) (DamageType :type Damage%20Type%20Object%20Reference) (InstigatedBy :type Controller%20Object%20Reference) (DamageCauser :type Actor%20Object%20Reference))
  (Variables|Default|SetHealth (- (Variables|Default|GetHealth) Damage))
  (if (< (Variables|Default|GetHealth) 0.0)
    (Variables|Default|SetIs%20True true)
    (Actor|DestroyActor)))

(fn ConstructionScript)